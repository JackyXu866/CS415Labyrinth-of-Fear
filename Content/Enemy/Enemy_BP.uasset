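; Enemy Blueprint that chases the player and repeatedly damages them on contact.
; ChasePlayer starts on BeginPlay or when PawnSensing sees a pawn, running AI Move To and retrying after successful moves.
; A lit player lighter switches to a move with a larger acceptance radius that only retries if the path to the player isn't very short.
; Capsule overlap drives a self-repeating, delayed damage loop until contact ends.
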(event `self.ReceiveBeginPlay`
  (`self.ChasePlayer`))

(event `self.CapsuleComponent.OnComponentBeginOverlap`
  (params (OverlappedComponent :type "PrimitiveComponent Object Reference") (OtherActor :type "Actor Object Reference") (OtherComp :type "PrimitiveComponent Object Reference") (OtherBodyIndex :type Integer) (bFromSweep :type Boolean) (SweepResult :type "HitResult Structure (by ref)"))
  (if (== OtherActor (`GameplayStatics.GetPlayerPawn` 0))
    (set `self.Overlapping` true)
    (`self.GetDamage`)))

(event `GetDamage`
  (if (`self.Overlapping`)
    (bind _asmaster (`/Game/HorrorEngine/Blueprints/Core/HorrorEngineFunctions.GetPlayer`))
    (`/Game/HorrorEngine/HorrorEngine.GetDamage` :`self` _asmaster :`DamagePoint` 30.0)
    (`KismetSystemLibrary.Delay` 2.0)
    (`self.GetDamage`)))

(event `self.CapsuleComponent.OnComponentEndOverlap`
  (params (OverlappedComponent :type "PrimitiveComponent Object Reference") (OtherActor :type "Actor Object Reference") (OtherComp :type "PrimitiveComponent Object Reference") (OtherBodyIndex :type Integer))
  (if (== OtherActor (`GameplayStatics.GetPlayerPawn` 0))
    (set `self.Overlapping` false)))

(event `ChasePlayer`
  (bind _returnvalue (`GameplayStatics.GetPlayerCharacter` 0))
  (bind _asmaster (`/Game/HorrorEngine/Blueprints/Core/HorrorEngineFunctions.GetPlayer`))
  (if (`/Game/HorrorEngine/HorrorEngine.HasLighter` _asmaster)
    (if (`/Game/HorrorEngine/HorrorEngine.LighterOff` _asmaster)
      (`|AIMoveTo` self (0.0 0.0 0.0) _returnvalue :!label _label
        (:`OnSuccess`
          (`KismetSystemLibrary.Delay` 1.0)
          (`self.ChasePlayer`)))
      (else
        (`|AIMoveTo` self (0.0 0.0 0.0) _returnvalue 100.0 true
          (:`OnSuccess`
            (if (not (< (`NavigationSystemV1.GetPathLength` (`self.K2_GetActorLocation` self) (`self.K2_GetActorLocation` _returnvalue) null null) 50.0))
              (`KismetSystemLibrary.Delay` 1.0)
              (`self.ChasePlayer`))))))
    (else
      (goto _label))))

(event `self.PawnSensing.OnSeePawn`
  (params (Pawn :type "Pawn Object Reference"))
  (`self.ChasePlayer`))

(fn `UserConstructionScript`)